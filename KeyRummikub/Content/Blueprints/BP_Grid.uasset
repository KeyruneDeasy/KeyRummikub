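; BP_Grid is a grid actor in a Rummikub game that handles bounds setup and debug display.
; On BeginPlay it sizes its box component from grid size and spacing, and every Tick it draws debug grid lines.
; The construction script places two cubes at the world bounds' min and max corners.
; A helper returns the cast Rummikub game state; coordinate debug drawing is left unwired.
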(event `self.ReceiveBeginPlay`
  (`BoxComponent.SetBoxExtent` (`self.Box`) (`KismetMathLibrary.MakeVector` (* (`KismetMathLibrary.Conv_IntToDouble` (`self.GetGridSizeX`)) (`self.GetGridSpacingX`) 0.5) (* (`KismetMathLibrary.Conv_IntToDouble` (`self.GetGridSizeY`)) (`self.GetGridSpacingY`) 0.5) 20.0) true))

(event `self.ReceiveTick`
  (params (DeltaSeconds :type "Float (single-precision)"))
  (`self.EventDrawGridLines`))

(event `EventDrawGridLines`
  (`self.DebugDrawGridLines`))

(fn `GetRummiGameState`
  (returns (GameState :type "KeyRummikubGameState Object Reference"))
  (bind _askey_rummikub_game_state (cast `KeyRummikubGameState` (`GameplayStatics.GetGameState`)))
  (return _askey_rummikub_game_state))

(fn `UserConstructionScript`
  (bind (_outmin _outmax) (`self.GetWorldBounds`))
  (`SceneComponent.K2_SetWorldLocation` (`self.Cube`) _outmin false false)
  (`SceneComponent.K2_SetWorldLocation` (`self.Cube1`) _outmax false false))