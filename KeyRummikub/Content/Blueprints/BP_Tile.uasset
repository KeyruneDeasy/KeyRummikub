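; BP_Tile is a tile actor for a Rummikub game that carries a number and a color in TileInfo.
; It starts hidden, teleports to its cell and shows itself when placed into the grid, and hides again when removed.
; While visible, it draws its number every tick as a debug string at DebugStringLocator, tinted by a color looked up from BP_KeyRummikubGameState.
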(event `self.ReceiveBeginPlay`
  (`SceneComponent.SetVisibility` (`self.DefaultSceneRoot`) false true))

(event `self.ReceiveTick`
  (params (DeltaSeconds :type "Float (single-precision)"))
  (if (`SceneComponent.IsVisible` (`self.DefaultSceneRoot`))
    (`self.DebugDrawValue`)))

(event `self.OnPlacedIntoGrid`
  (params (InGridCellLocation :type "Vector Structure (by ref)"))
  (`parent.OnPlacedIntoGrid` InGridCellLocation)
  (`self.K2_SetActorLocation` InGridCellLocation false true)
  (`SceneComponent.SetVisibility` (`self.DefaultSceneRoot`) true true))

(event `self.OnRemovedFromGrid`
  (`SceneComponent.SetVisibility` (`self.DefaultSceneRoot`) false true))

(fn `DebugDrawValue`
  (`KismetSystemLibrary.DrawDebugString` (`SceneComponent.K2_GetComponentLocation` (`self.DebugStringLocator`)) (`KismetStringLibrary.Conv_IntToString` (`.Number` (break `RummiTile` (`self.TileInfo`)))) null (`KismetMathLibrary.Conv_ColorToLinearColor` (`self.GetColor`))))

(fn `GetColor`
  (returns (Output :type "Color Structure"))
  (bind _asbp_key_rummikub_game_state (cast `/Game/Blueprints/BP_KeyRummikubGameState` (`GameplayStatics.GetGameState`)))
  (return (`/Game/Blueprints/BP_KeyRummikubGameState.GetColor` _asbp_key_rummikub_game_state (`.Color` (break `RummiTile` (`self.TileInfo`))))))

(fn `UserConstructionScript`)