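; Game state Blueprint for a Rummikub-style tile game, providing turn-end, color lookup and deck debug helpers.
; EndTurn draws from the deck into hand 0.
; GetColor maps an index to the Colors array, falling back to opaque white when the index is invalid.
; PrintDeck prints each deck tile's number on screen in its color, but its event graph call is disconnected.
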(event `self.ReceiveTick`
  (params (DeltaSeconds :type "Float (single-precision)")))

(fn `EndTurn`
  (`self.DrawCardFromDeckToHand` 0))

(fn `GetColor`
  (params (Index :type Integer))
  (returns (Output :type "Color Structure"))
  (bind _colors (`self.Colors`))
  (if (`KismetArrayLibrary.Array_IsValidIndex` _colors Index)
    (return (`|GetArrayItem` _colors Index))
    (else
      (return (make `Color` 255 255 255 255)))))

(fn `PrintDeck`
  (locals (String :type "Object Object Reference"))
  (for _array_element (`.Tiles` (break `RummiTileArray` (`.Deck` (break `RummiTable` (`self.Table`)))))
    (bind (_color _number) (break `RummiTile` _array_element))
    (`KismetSystemLibrary.PrintString` (`KismetStringLibrary.Conv_IntToString` _number) true true (`KismetMathLibrary.Conv_ColorToLinearColor` (`self.GetColor` _color)) 0.0)))

(fn `UserConstructionScript`)