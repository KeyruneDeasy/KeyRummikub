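; Player controller that lets the player drag grid tiles with the mouse.
; A left-click trace under the cursor asks the hit BP_Grid for the tile at that point and stores it with the hit point, normal and grab offset.
; Each tick, the mouse ray is projected onto the plane of that initial hit and the tile teleports there minus the offset, until release clears it.
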(event `self.ReceiveTick`
  (params (DeltaSeconds :type "Float (single-precision)"))
  (`self.UpdateHeldTile`))

(event `Key|LeftMouseButton`
  (params (Key :type "Key Structure"))
  (bind (_bblockinghit _binitialoverlap _time _distance _location _impactpoint _normal _impactnormal _physmat _hitactor) (`GameplayStatics.BreakHitResult` (`self.GetHitResultUnderCursorByChannel` "TraceTypeQuery3")))
  (:`Pressed`
    (if _bblockinghit
      (bind _asbp_grid (cast `/Game/Blueprints/BP_Grid` _hitactor))
      (bind _output_get (set `self.HeldTile` (`RummiGrid.GetTileActorAtWorldLocation` _asbp_grid _impactpoint)))
      (`/Engine/EditorBlueprintResources/StandardMacros.IsValid` _output_get
        (:`Is Valid`
          (bind _output_get_2 (set `self.HeldTileInitialHitLocation` _impactpoint))
          (set `self.HeldTileInitialHitNormal` _normal)
          (set `self.HeldTileInitialHitOffset` (- _output_get_2 (`self.K2_GetActorLocation` (`self.HeldTile`))))))))
  (:`Released`
    (set `self.HeldTile` null) ; Set to NULL
  ))

(fn `UpdateHeldTile`
  (bind (_worldlocation _worlddirection _returnvalue) (`self.DeprojectMousePositionToWorld`))
  (`/Engine/EditorBlueprintResources/StandardMacros.IsValid` (`self.HeldTile`)
    (:`Is Valid`
      (if _returnvalue
        (bind _returnvalue_2 (`KeyUtil.TraceToPlane` _worldlocation _worlddirection (`self.HeldTileInitialHitLocation`) (`self.HeldTileInitialHitNormal`)))
        (`self.K2_SetActorLocation` (`self.HeldTile`) (- _returnvalue_2 (`self.HeldTileInitialHitOffset`)) false true)))))

(fn `UserConstructionScript`)